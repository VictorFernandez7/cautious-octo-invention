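; BP_PlayerCharacter is the player character Blueprint, with input for world-axis movement and stick-style facing.
; MoveForward and MoveRight add movement along fixed world X and Y, independent of camera or control rotation.
; LookUp and LookRight share one chain that builds an XY vector from axis input.
; Past a 0.25 length dead zone, that vector's direction directly sets the controller's control rotation.
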(event `InputAxis|MoveForward`
  (params (AxisValue :type "Float (single-precision)"))
  ;[0.655 1 0.8339] Movement
  (`self.AddMovementInput` (1.0 0.0 0.0) AxisValue))

(event `InputAxis|MoveRight`
  (params (AxisValue :type "Float (single-precision)"))
  ;[0.655 1 0.8339] Movement
  (`self.AddMovementInput` (0.0 1.0 0.0) AxisValue))

(event `InputAxis|LookUp`
  (params (AxisValue :type "Float (single-precision)"))
  ;[1 0.6969 0.2395] Look
  (bind _returnvalue (`KismetMathLibrary.MakeVector` AxisValue (stale `InputAxis|LookRight` AxisValue)))
  (if (> (`KismetMathLibrary.VSize` _returnvalue) 0.25) :!label _label
    (`Controller.SetControlRotation` (`self.GetController`) (`KismetMathLibrary.Conv_VectorToRotator` _returnvalue))))

(event `InputAxis|LookRight`
  (params (AxisValue :type "Float (single-precision)"))
  ;[1 0.6969 0.2395] Look
  (goto _label))

(fn `UserConstructionScript`)