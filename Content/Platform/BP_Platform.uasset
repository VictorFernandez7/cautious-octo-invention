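; BP_Platform is a moving platform that travels through an array of waypoint actors in a continuous loop.
; BeginPlay records the start location, the last waypoint index and a first target of zero.
; Tick plays the PlatformSpeed timeline, which lerps the actor from the recorded location to the current waypoint without sweeping.
; On arrival, Tick records the new start, advances or wraps the index, and restarts the timeline.
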(event `self.ReceiveBeginPlay`
  ;[0 0.9546 1] Begin Play
  (`|ExecutionSequence`
    (:`then_0`
      (set `self.InitialPosition` (`self.K2_GetActorLocation`)))
    (:`then_1`
      (set `self.Max Waypoints` (- (`KismetArrayLibrary.Array_Length` (`self.Waypoints`)) 1)))
    (:`then_2`
      (set `self.Current Waypoint` 0))))

(event `self.ReceiveTick`
  (params (DeltaSeconds :type "Float (single-precision)"))
  ;[0.5713 1 0.383] Tick
  (if (!= (`self.K2_GetActorLocation`) (`self.K2_GetActorLocation` (`|GetArrayItem` (`self.Waypoints`) (`self.Current Waypoint`))))
    (bind (_direction _time) (`Timeline|Platform Speed` :!label _label)
      (:`Update`
        (`self.K2_SetActorLocation` (`KismetMathLibrary.VLerp` (`self.InitialPosition`) (`self.K2_GetActorLocation` (`|GetArrayItem` (`self.Waypoints`) (`self.Current Waypoint`))) _time))))
    (else
      (set `self.InitialPosition` (`self.K2_GetActorLocation`))
      (if (< (`self.Current Waypoint`) (`self.Max Waypoints`))
        (set `self.Current Waypoint` (+ (`self.Current Waypoint`) 1))
        (goto _label :!via `PlayFromStart`)
        (else
          (set `self.Current Waypoint` 0)
          (goto _label :!via `PlayFromStart`))))))

(fn `UserConstructionScript`)